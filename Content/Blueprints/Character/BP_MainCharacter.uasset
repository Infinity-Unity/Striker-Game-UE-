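; Player shooter character with Enhanced Input movement, sprint and jump, spawning a socket-attached weapon and HUD on BeginPlay.
; Aiming switches to controller-yaw rotation, shows a crosshair and slides the camera through a timeline.
; Firing requires aiming and repeats via DoOnce and delay, tracing from camera, then muzzle toward that point with debug drawing, but applies no damage.
; Ammo counters drive empty-gun sound or fire montage with camera shake, and reloading draws from reserves.
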(event `EnhancedInput|/Game/_Core/Inputs/Action/IA_Sprint`
  (params (ActionValue :type Boolean) (ElapsedSeconds :type "Float (double-precision)") (TriggeredSeconds :type "Float (double-precision)") (InputAction :type "InputAction Object Reference" :default "/Game/_Core/Inputs/Action/IA_Sprint.IA_Sprint"))
  (bind _charactermovement (`self.CharacterMovement`))
  ; Sprint
  (:`Started`
    (set `CharacterMovementComponent.MaxWalkSpeed` 500.0 _charactermovement)
    (set `self.bIsSprint` true))
  (:`Canceled`
    (set `CharacterMovementComponent.MaxWalkSpeed` 250.0 _charactermovement :!label _label)
    (set `self.bIsSprint` false))
  (:`Completed`
    (goto _label)))

(event `EnhancedInput|/Game/_Core/Inputs/Action/IA_Jump`
  (params (ActionValue :type Boolean) (ElapsedSeconds :type "Float (double-precision)") (TriggeredSeconds :type "Float (double-precision)") (InputAction :type "InputAction Object Reference" :default "/Game/_Core/Inputs/Action/IA_Jump.IA_Jump"))
  ; Jumping
  (:`Started`
    (if (<= (`KismetMathLibrary.VSize` (`self.GetVelocity`)) 10.0)
      (`self.Jump`)
      (set `self.bIsJumping` true))))

(event `EnhancedInput|/Game/_Core/Inputs/Action/IA_Look`
  (params (ActionValue :type "Vector2D Structure") (ElapsedSeconds :type "Float (double-precision)") (TriggeredSeconds :type "Float (double-precision)") (InputAction :type "InputAction Object Reference" :default "/Game/_Core/Inputs/Action/IA_Look.IA_Look"))
  ; Look
  (:`Triggered`
    (`self.AddControllerYawInput` ActionValue_X)
    (`self.AddControllerPitchInput` ActionValue_Y)))

(event `self.ReceiveBeginPlay`
  ; BeginPlay
  (`|ExecutionSequence`
    (:`then_0`
      (bind _asplayer_controller (cast `PlayerController` (`self.GetController`)))
      (message `EnhancedInputSubsystemInterface.AddMappingContext` (pcsubsystem `EnhancedInputLocalPlayerSubsystem` _asplayer_controller) "/Game/_Core/Inputs/IMC_Player.IMC_Player" 0 (struct)))
    (:`then_1`
      (bind _returnvalue (`|SpawnActorFromClass` "/Game/Blueprints/Character/BP_Weapon.BP_Weapon_C" (`SceneComponent.GetSocketTransform` (`self.Mesh`) "WeaponSocket" "RTS_World") "Undefined" "MultiplyWithRoot" null null))
      (bind _output_get (set `self.BP_Weapon` _returnvalue))
      (`self.K2_AttachToComponent` _output_get (`self.Mesh`) "WeaponSocket" "SnapToTarget" "SnapToTarget" "SnapToTarget" true))
    (:`then_2`
      (bind _returnvalue_2 (`|CreateWidget` "/Game/UI/Widgets/HUD/WBP_Crosshair.WBP_Crosshair_C"))
      (set `self.WBP_Crosshair` _returnvalue_2)
      (bind _returnvalue_3 (`|CreateWidget` "/Game/UI/Widgets/HUD/WBP_Main.WBP_Main_C"))
      (bind _output_get_2 (set `self.WBP_Main` _returnvalue_3))
      (`UserWidget.AddToViewport` _output_get_2 0))))

(event `EnhancedInput|/Game/_Core/Inputs/Action/IA_Move`
  (params (ActionValue :type "Vector2D Structure") (ElapsedSeconds :type "Float (double-precision)") (TriggeredSeconds :type "Float (double-precision)") (InputAction :type "InputAction Object Reference" :default "/Game/_Core/Inputs/Action/IA_Move.IA_Move"))
  (bind (_returnvalue_roll _returnvalue_pitch _returnvalue_yaw) (`KismetMathLibrary.BreakRotator` (`self.GetControlRotation`)))
  (bind (_returnvalue_roll_2 _returnvalue_pitch_2 _returnvalue_yaw_2) (`KismetMathLibrary.BreakRotator` (`self.GetControlRotation`)))
  ; Input
  (:`Triggered`
    (`self.AddMovementInput` (`KismetMathLibrary.GetRightVector` (`KismetMathLibrary.MakeRotator` _returnvalue_roll_2 0.0 _returnvalue_yaw_2)) ActionValue_X)
    (`self.AddMovementInput` (`KismetMathLibrary.GetForwardVector` (`KismetMathLibrary.MakeRotator` 0.0 0.0 _returnvalue_yaw)) ActionValue_Y)))

(event `self.OnLanded`
  (params (Hit :type "HitResult Structure (by ref)"))
  ; Jumping
  (set `self.bIsJumping` false))

(event `EnhancedInput|/Game/_Core/Inputs/Action/IA_Aiming`
  (params (ActionValue :type Boolean) (ElapsedSeconds :type "Float (double-precision)") (TriggeredSeconds :type "Float (double-precision)") (InputAction :type "InputAction Object Reference" :default "/Game/_Core/Inputs/Action/IA_Aiming.IA_Aiming"))
  (bind (_relativelocation_x _relativelocation_y _relativelocation_z) (`KismetMathLibrary.BreakVector` (`SceneComponent.RelativeLocation` (`self.Camera`))))
  ; Aim
  (:`Started`
    (`self.Aim`)
    (bind (_direction _zoomcrosshairtrack) (`Timeline|TL_Zoom` :!label _label_2)
      (:`Update`
        (`SceneComponent.K2_SetRelativeLocation` (`self.Camera`) (`KismetMathLibrary.MakeVector` (`KismetMathLibrary.Lerp` 0.0 130.0 _zoomcrosshairtrack) _relativelocation_y _relativelocation_z) false false))))
  (:`Canceled`
    (`self.StopAim` :!label _label_3)
    (goto _label_2 :!via `Reverse`))
  (:`Completed`
    (goto _label_3)))

(event `EnhancedInput|/Game/_Core/Inputs/Action/IA_Shoot`
  (params (ActionValue :type Boolean) (ElapsedSeconds :type "Float (double-precision)") (TriggeredSeconds :type "Float (double-precision)") (InputAction :type "InputAction Object Reference" :default "/Game/_Core/Inputs/Action/IA_Shoot.IA_Shoot"))
  ; Shoot
  (:`Triggered`
    (if (`self.bIsAiming`)
      (`/Engine/EditorBlueprintResources/StandardMacros.DoOnce` false :!label _label_4
        (:`Completed`
          (`self.LineTrace`)
          (`self.AmmoCountCalculate`)
          (`self.PlaySoundEmptyAkPlayMonatge`
            (:`NewParam2`
              (`KismetSystemLibrary.Delay` 0.1)
              (goto _label_4 :!via `Reset`)))))))
  (:`Canceled`
    (`self.StopAnimMontage` "/Game/Art/Characters/Animations/Fire_Rifle_Ironsights_Montage.Fire_Rifle_Ironsights_Montage" :!label _label_5)
    (goto _label_4 :!via `Reset`))
  (:`Completed`
    (goto _label_5)))

(event `EnhancedInput|/Game/_Core/Inputs/Action/IA_FindActorPressed`
  (params (ActionValue :type Boolean) (ElapsedSeconds :type "Float (double-precision)") (TriggeredSeconds :type "Float (double-precision)") (InputAction :type "InputAction Object Reference" :default "/Game/_Core/Inputs/Action/IA_FindActorPressed.IA_FindActorPressed"))
  ; Fire
  (:`Started`
    (`self.FireObject`)))

(event `EnhancedInput|/Game/_Core/Inputs/Action/IA_Reload`
  (params (ActionValue :type Boolean) (ElapsedSeconds :type "Float (double-precision)") (TriggeredSeconds :type "Float (double-precision)") (InputAction :type "InputAction Object Reference" :default "/Game/_Core/Inputs/Action/IA_Reload.IA_Reload"))
  ; Reload
  (:`Started`
    (`self.ReloadGun`)))

(event `self.ReceiveTick`
  (params (DeltaSeconds :type "Float (single-precision)"))
  (`KismetSystemLibrary.PrintString` (`KismetStringLibrary.Conv_BoolToString` (`self.bIsSprint`)) true true (struct :`G` 0.66 :`B` 1.0 :`A` 1.0) 2.0 "28"))

(fn `Aim`
  (set `CharacterMovementComponent.bOrientRotationToMovement` false (`self.CharacterMovement`))
  (set `self.bIsAiming` true)
  (set `self.bUseControllerRotationYaw` true)
  (`UserWidget.AddToViewport` (`self.WBP_Crosshair`) 0)
  (`UserWidget.PlayAnimationForward` (`self.WBP_Crosshair`) (`/Game/UI/Widgets/HUD/WBP_Crosshair.ZoomCrosshair` (`self.WBP_Crosshair`)) 1.0 false))

(fn `AmmoCountCalculate`
  (set `self.AmmoCount` (`KismetMathLibrary.Clamp` (- (`self.AmmoCount`) 1) 0 30)))

(fn `FireObject`)

(fn `LineTrace`
  (locals (NewLocalVar :type "Vector Structure" :default (0.0 0.0 0.0)))
  (bind _returnvalue (`GameplayStatics.GetPlayerCameraManager` 0))
  (bind _returnvalue_2 (`self.K2_GetActorLocation` _returnvalue))
  (if (not (!= (`self.TotalAmmo`) 0))
    (set `self.bIsNeedTotalAmmo` true))
  (if (!= (`self.AmmoCount`) 0)
    (set `self.WeaponLocation` (`SceneComponent.K2_GetComponentLocation` (`/Game/Blueprints/Character/BP_Weapon.ArrowBullet` (`self.BP_Weapon`))))
    (bind _outhit (`KismetSystemLibrary.LineTraceSingle` _returnvalue_2 (+ _returnvalue_2 (* (`self.GetActorForwardVector` _returnvalue) 10000.0)) "TraceTypeQuery1"))
    (if (`GameplayStatics.BreakHitResult` _outhit)
      (`KismetSystemLibrary.LineTraceSingle` :`Start` (`self.WeaponLocation`) :`End` (`.Location` (`GameplayStatics.BreakHitResult` _outhit)) :`TraceChannel` "TraceTypeQuery1" :`DrawDebugType` "ForDuration")
      (`KismetSystemLibrary.PrintString` "on hit" true true (struct :`G` 0.66 :`B` 1.0 :`A` 1.0) 0.1 "30")
      (else
        (`KismetSystemLibrary.LineTraceSingle` :`Start` (`self.WeaponLocation`) :`End` (`.TraceEnd` (`GameplayStatics.BreakHitResult` _outhit)) :`TraceChannel` "TraceTypeQuery1" :`DrawDebugType` "ForDuration")))
    (`GameplayStatics.SpawnSound2D` "/Game/Audio/Sounds/Ak47ShootSound.Ak47ShootSound" 1.0 (`KismetMathLibrary.FClamp` (`KismetMathLibrary.RandomFloat`) 0.8) 0.0 null)
    (`/Game/Blueprints/Character/BP_Weapon.FireEffect` (`self.BP_Weapon`))
    (else
      (set `self.bIsNeedAmmo` true))))

(fn `ReloadGun`
  (bind _returnvalue (- (`self.MaxAmmo`) (`self.AmmoCount`)))
  (if (and (!= (`self.AmmoCount`) (`self.MaxAmmo`)) (!= (`self.TotalAmmo`) 0))
    (if (< _returnvalue (`self.TotalAmmo`))
      (set `self.TotalAmmo` (- (`self.TotalAmmo`) _returnvalue))
      (set `self.AmmoCount` (+ _returnvalue (`self.AmmoCount`)))
      (set `self.bIsNeedAmmo` false)
      (else
        (set `self.AmmoCount` (+ (`self.AmmoCount`) (`self.TotalAmmo`)))
        (set `self.TotalAmmo` 0)
        (set `self.bIsNeedAmmo` false)))))

(fn `StopAim`
  (set `CharacterMovementComponent.bOrientRotationToMovement` true (`self.CharacterMovement`))
  (set `self.bIsAiming` false)
  (set `self.bUseControllerRotationYaw` false)
  (`Widget.RemoveFromParent` (`self.WBP_Crosshair`)))

(fn `UserConstructionScript`)