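; Player character with Enhanced Input movement, sprint, jump from near standstill, and an aim-gated rifle with ammo and reload.
; BeginPlay attaches BP_Weapon to the hand mesh's WeaponSocket and creates WBP_HUD, shown only while aiming alongside controller-yaw rotation and a timeline camera zoom.
; Shooting is delay-throttled, decrements ammo, then traces from camera to find the target and from muzzle toward it with debug drawing.
; No damage is applied; FireObject is an empty stub.
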(event `EnhancedInput|/Game/Player/Input/Action/IA_Sprint`
  (params (ActionValue :type Boolean) (ElapsedSeconds :type "Float (double-precision)") (TriggeredSeconds :type "Float (double-precision)") (InputAction :type "InputAction Object Reference" :default "/Game/Player/Input/Action/IA_Sprint.IA_Sprint"))
  (bind _charactermovement (`self.CharacterMovement`))
  ; Sprint
  (:`Started`
    (set `CharacterMovementComponent.MaxWalkSpeed` 500.0 _charactermovement)
    (set `self.bIsSprint` true))
  (:`Canceled`
    (set `CharacterMovementComponent.MaxWalkSpeed` 250.0 _charactermovement :!label _label)
    (set `self.bIsSprint` false))
  (:`Completed`
    (goto _label)))

(event `EnhancedInput|/Game/Player/Input/Action/IA_Jump`
  (params (ActionValue :type Boolean) (ElapsedSeconds :type "Float (double-precision)") (TriggeredSeconds :type "Float (double-precision)") (InputAction :type "InputAction Object Reference" :default "/Game/Player/Input/Action/IA_Jump.IA_Jump"))
  ; Jumping
  (:`Started`
    (if (<= (`KismetMathLibrary.VSize` (`self.GetVelocity`)) 10.0)
      (`self.Jump`)
      (set `self.bIsJumping` true))))

(event `EnhancedInput|/Game/Player/Input/Action/IA_Look`
  (params (ActionValue :type "Vector2D Structure") (ElapsedSeconds :type "Float (double-precision)") (TriggeredSeconds :type "Float (double-precision)") (InputAction :type "InputAction Object Reference" :default "/Game/Player/Input/Action/IA_Look.IA_Look"))
  ; Look
  (:`Triggered`
    (`self.AddControllerYawInput` ActionValue_X)
    (`self.AddControllerPitchInput` ActionValue_Y)))

(event `self.ReceiveBeginPlay`
  ; BeginPlay
  (`|ExecutionSequence`
    (:`then_0`
      (bind _asplayer_controller (cast `PlayerController` (`self.GetController`)))
      (message `EnhancedInputSubsystemInterface.AddMappingContext` (pcsubsystem `EnhancedInputLocalPlayerSubsystem` _asplayer_controller) "/Game/Player/Input/IMC_Player.IMC_Player" 0 (struct)))
    (:`then_1`
      (bind _returnvalue (`|SpawnActorFromClass` "/Game/Player/Blueprints/BP_Weapon.BP_Weapon_C" (`SceneComponent.GetSocketTransform` (`self.Mesh`) "WeaponSocket" "RTS_World") "Undefined" "MultiplyWithRoot" null null))
      (bind _output_get (set `self.BP_Weapon` _returnvalue))
      (`self.K2_AttachToComponent` _output_get (`self.Mesh`) "WeaponSocket" "SnapToTarget" "SnapToTarget" "SnapToTarget" true))
    (:`then_2`
      (bind _returnvalue_2 (`|CreateWidget` "/Game/Widgets/WBP_HUD.WBP_HUD_C"))
      (set `self.WBP_HUD` _returnvalue_2))))

(event `EnhancedInput|/Game/Player/Input/Action/IA_Move`
  (params (ActionValue :type "Vector2D Structure") (ElapsedSeconds :type "Float (double-precision)") (TriggeredSeconds :type "Float (double-precision)") (InputAction :type "InputAction Object Reference" :default "/Game/Player/Input/Action/IA_Move.IA_Move"))
  (bind (_returnvalue_roll _returnvalue_pitch _returnvalue_yaw) (`KismetMathLibrary.BreakRotator` (`self.GetControlRotation`)))
  (bind (_returnvalue_roll_2 _returnvalue_pitch_2 _returnvalue_yaw_2) (`KismetMathLibrary.BreakRotator` (`self.GetControlRotation`)))
  ; Input
  (:`Triggered`
    (`self.AddMovementInput` (`KismetMathLibrary.GetRightVector` (`KismetMathLibrary.MakeRotator` _returnvalue_roll_2 0.0 _returnvalue_yaw_2)) ActionValue_X)
    (`self.AddMovementInput` (`KismetMathLibrary.GetForwardVector` (`KismetMathLibrary.MakeRotator` 0.0 0.0 _returnvalue_yaw)) ActionValue_Y)))

(event `self.OnLanded`
  (params (Hit :type "HitResult Structure (by ref)"))
  ; Jumping
  (set `self.bIsJumping` false))

(event `EnhancedInput|/Game/Player/Input/Action/IA_Aiming`
  (params (ActionValue :type Boolean) (ElapsedSeconds :type "Float (double-precision)") (TriggeredSeconds :type "Float (double-precision)") (InputAction :type "InputAction Object Reference" :default "/Game/Player/Input/Action/IA_Aiming.IA_Aiming"))
  (bind (_relativelocation_x _relativelocation_y _relativelocation_z) (`KismetMathLibrary.BreakVector` (`SceneComponent.RelativeLocation` (`self.Camera`))))
  ; Aim
  (:`Started`
    (`self.Aim`)
    (bind (_direction _zoomcrosshairtrack) (`Timeline|TL_Zoom` :!label _label_2)
      (:`Update`
        (`SceneComponent.K2_SetRelativeLocation` (`self.Camera`) (`KismetMathLibrary.MakeVector` (`KismetMathLibrary.Lerp` 0.0 130.0 _zoomcrosshairtrack) _relativelocation_y _relativelocation_z) false false))))
  (:`Canceled`
    (`self.StopAim` :!label _label_3)
    (goto _label_2 :!via `Reverse`))
  (:`Completed`
    (goto _label_3)))

(event `EnhancedInput|/Game/Player/Input/Action/IA_Shoot`
  (params (ActionValue :type Boolean) (ElapsedSeconds :type "Float (double-precision)") (TriggeredSeconds :type "Float (double-precision)") (InputAction :type "InputAction Object Reference" :default "/Game/Player/Input/Action/IA_Shoot.IA_Shoot"))
  ; Shoot
  (:`Triggered`
    (if (`self.bIsAiming`)
      (`/Engine/EditorBlueprintResources/StandardMacros.DoOnce` false :!label _label_4
        (:`Completed`
          (`self.AmmoCountCalculate`)
          (`self.LineTrace`)
          (if (== (`self.AmmoCount`) 0)
            (set `self.bIsNeedAmmo` true)
            (`GameplayStatics.SpawnSound2D` "/Game/Sounds/noammo.noammo" 1.0 1.0 0.0 null))
          (`KismetSystemLibrary.Delay` 0.1)
          (goto _label_4 :!via `Reset`))))))

(event `EnhancedInput|/Game/Player/Input/Action/IA_FindActorPressed`
  (params (ActionValue :type Boolean) (ElapsedSeconds :type "Float (double-precision)") (TriggeredSeconds :type "Float (double-precision)") (InputAction :type "InputAction Object Reference" :default "/Game/Player/Input/Action/IA_FindActorPressed.IA_FindActorPressed"))
  ; Fire
  (:`Started`
    (`self.FireObject`)))

(event `EnhancedInput|/Game/Player/Input/Action/IA_Reload`
  (params (ActionValue :type Boolean) (ElapsedSeconds :type "Float (double-precision)") (TriggeredSeconds :type "Float (double-precision)") (InputAction :type "InputAction Object Reference" :default "/Game/Player/Input/Action/IA_Reload.IA_Reload"))
  ; Shoot
  ;; Reload
  (:`Started`
    (`self.ReloadGun`)))

(event `self.ReceiveTick`
  (params (DeltaSeconds :type "Float (single-precision)"))
  (`KismetSystemLibrary.PrintString` (`KismetStringLibrary.Conv_BoolToString` (`self.bIsSprint`)) true true (struct :`G` 0.66 :`B` 1.0 :`A` 1.0) 2.0 "28"))

(fn `Aim`
  (set `self.bIsAiming` true)
  (set `self.bUseControllerRotationYaw` true)
  (`UserWidget.AddToViewport` (`self.WBP_HUD`) 0)
  (`UserWidget.PlayAnimationForward` (`self.WBP_HUD`) (`/Game/Widgets/WBP_HUD.ZoomCrosshair` (`self.WBP_HUD`)) 1.0 false))

(fn `AmmoCountCalculate`
  (set `self.AmmoCount` (`KismetMathLibrary.Clamp` (- (`self.AmmoCount`) 1) 0 30)))

(fn `FireObject`)

(fn `LineTrace`
  (bind _returnvalue (`GameplayStatics.GetPlayerCameraManager` 0))
  (bind _returnvalue_2 (`self.K2_GetActorLocation` _returnvalue))
  (bind _returnvalue_3 (`SceneComponent.K2_GetComponentLocation` (`/Game/Player/Blueprints/BP_Weapon.ArrowBullet` (`self.BP_Weapon`))))
  (if (!= (`self.TotalAmmo`) 0)
    (if (!= (`self.AmmoCount`) 0)
      (`GameplayStatics.SpawnSound2D` "/Game/Sounds/Ak47ShootSound.Ak47ShootSound" 1.0 (`KismetMathLibrary.FClamp` (`KismetMathLibrary.RandomFloat`) 0.8) 0.0 null)
      (bind _outhit (`KismetSystemLibrary.LineTraceSingle` _returnvalue_2 (+ _returnvalue_2 (* (`self.GetActorForwardVector` _returnvalue) 50000.0)) "TraceTypeQuery1"))
      (if (`GameplayStatics.BreakHitResult` _outhit)
        (`KismetSystemLibrary.LineTraceSingle` :`Start` _returnvalue_3 :`End` (`.Location` (`GameplayStatics.BreakHitResult` _outhit)) :`TraceChannel` "TraceTypeQuery1" :`DrawDebugType` "ForDuration")
        (else
          (`KismetSystemLibrary.LineTraceSingle` :`Start` _returnvalue_3 :`End` (`.TraceEnd` (`GameplayStatics.BreakHitResult` _outhit)) :`TraceChannel` "TraceTypeQuery1" :`DrawDebugType` "ForDuration"))))
    (else
      (set `self.bIsNeedTotalAmmo` true))))

(fn `ReloadGun`
  (bind _returnvalue (- (`self.MaxAmmo`) (`self.AmmoCount`)))
  (if (and (!= (`self.AmmoCount`) (`self.MaxAmmo`)) (!= (`self.TotalAmmo`) 0))
    (if (< _returnvalue (`self.TotalAmmo`))
      (set `self.TotalAmmo` (- (`self.TotalAmmo`) _returnvalue))
      (set `self.AmmoCount` (+ _returnvalue (`self.AmmoCount`)))
      (set `self.bIsNeedAmmo` false)
      (else
        (set `self.AmmoCount` (+ (`self.AmmoCount`) (`self.TotalAmmo`)))
        (set `self.TotalAmmo` 0)
        (set `self.bIsNeedAmmo` false)))))

(fn `StopAim`
  (set `self.bIsAiming` false)
  (set `self.bUseControllerRotationYaw` false)
  (`Widget.RemoveFromParent` (`self.WBP_HUD`)))

(fn `UserConstructionScript`)